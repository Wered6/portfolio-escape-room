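; Base interactable cabinet door that swings open and closed when the player interacts, unless it is locked.
; An interact press checks the LockComponent: a locked door plays a TryOpen timeline rattle, while an unlocked one alternates playing and reversing the Open timeline via FlipFlop.
; Both timelines drive DoorMesh yaw scaled by angle variables.
; The door mesh registers for outlining, and WidgetAttachment anchors the interaction widget.
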(event EventInteractPressTriggered
  (|CallParentFunction)
  (if (Variables|/Script/EscapeRoom.ERLockComponent|GetbIsLocked (Variables|Default|GetLockComponent))
    (bind _rotation (Timeline|TryOpen PlayFromStart)
      (:Update
        (Transformation|SetRelativeRotation (Variables|Default|GetDoorMesh) (Math|Rotator|MakeRotator 0.0 0.0 (* _rotation (Variables|Default|GetTryOpenAngle))) false false)))
    (else
      (Utilities|FlowControl|FlipFlop
        (:A
          (bind _rotation_2 (Timeline|Open Play)
            (:Update
              (Transformation|SetRelativeRotation (Variables|Default|GetDoorMesh) (Math|Rotator|MakeRotator 0.0 0.0 (* _rotation_2 (Variables|Default|GetOpenAngle))) false false))))
        (:B
          (Timeline|Open Reverse))))))

(event EventBeginPlay
  (Class|ERInteractableComponent|AddOutlineMeshComponent (Variables|Default|GetInteractableComponent) (Variables|Default|GetDoorMesh)))

(fn ConstructionScript)

(fn GetWidgetAttachmentComponent
  (return (Variables|Default|GetWidgetAttachment)))