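; Base interactable cabinet drawer that slides open and closed on interaction and respects a lock component.
; On begin play it registers the drawer mesh for outlining with the interactable component.
; When unlocked, a FlipFlop plays or reverses the Open timeline, while a locked drawer plays a TryOpen timeline instead.
; Both timelines drive the mesh's relative Y location, scaled by their own multiplier variables.
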(event EventBeginPlay
  (Class|ERInteractableComponent|AddOutlineMeshComponent (Variables|Default|GetInteractableComp) (Variables|Default|GetDrawerMesh)))

(event EventInteractPressTriggered
  (|CallParentFunction)
  (if (Variables|/Script/EscapeRoom.ERLockComponent|GetbIsLocked (Variables|Default|GetLockComponent))
    (bind _move (Timeline|TryOpen PlayFromStart)
      (:Update
        (Transformation|SetRelativeLocation (Variables|Default|GetDrawerMesh) (Math|Vector|MakeVector 0.0 (* _move (Variables|Default|GetTryOpenMultiplayer)) 0.0) false false)))
    (else
      (Utilities|FlowControl|FlipFlop
        (:A
          (bind _move_2 (Timeline|Open Play)
            (:Update
              (Transformation|SetRelativeLocation (Variables|Default|GetDrawerMesh) (Math|Vector|MakeVector 0.0 (* _move_2 (Variables|Default|GetOpenMultiplayer)) 0.0) false false))))
        (:B
          (Timeline|Open Reverse))))))

(fn ConstructionScript)

(fn GetWidgetAttachmentComponent
  (return (Variables|Default|GetWidgetAttachment)))