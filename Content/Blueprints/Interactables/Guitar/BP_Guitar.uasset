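; BP_Guitar is an interactable guitar prop that plays an acoustic guitar sound when the player interacts with it.
; On BeginPlay it registers the guitar mesh with its interactable component for outlining.
; An interact press runs the parent handler, plays the attenuated sound at the actor's location, then disables further interaction.
; It overrides GetWidgetAttachmentComponent to supply its own widget attachment point.
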(event EventBeginPlay
  (Class|ERInteractableComponent|AddOutlineMeshComponent (Variables|Default|GetInteractableComp) (Variables|Default|GetGuitar)))

(event EventInteractPressTriggered
  (|CallParentFunction)
  (Audio|PlaySoundatLocation "/Game/Blueprints/Interactables/Guitar/acoustic_guitar.acoustic_guitar" (Transformation|GetActorLocation) "0, 0, 0" 1.0 1.0 0.0 "/Game/Blueprints/Interactables/Guitar/AT_Guitar.AT_Guitar" 0 0 0)
  (Class|ERInteractInterface|SetCanInteract false))

(fn ConstructionScript)

(fn GetWidgetAttachmentComponent
  (return (Variables|Default|GetWidgetAttachment)))