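; BP_OldRadio is an interactable old radio prop that plays a sound once when the player presses interact.
; On BeginPlay it registers its case mesh with the InteractableComponent as an outline mesh, and it supplies its own widget attachment component.
; Interacting runs the parent logic, plays the clip at the radio's location with the guitar attenuation settings, then disables further interaction.
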(event EventInteractPressTriggered
  (|CallParentFunction)
  (Audio|PlaySoundatLocation "/Game/Blueprints/Interactables/OldRadio/OldRadioTechlandJuniorProgrammer.OldRadioTechlandJuniorProgrammer" (Transformation|GetActorLocation) "0, 0, 0" 1.0 1.0 0.0 "/Game/Blueprints/Interactables/Guitar/AT_Guitar.AT_Guitar" 0 0 0)
  (Class|ERInteractInterface|SetCanInteract false))

(event EventBeginPlay
  (Class|ERInteractableComponent|AddOutlineMeshComponent (Variables|Default|GetInteractableComponent) (Variables|Default|GetCaseMesh)))

(fn ConstructionScript)

(fn GetWidgetAttachmentComponent
  (return (Variables|Default|GetWidgetAttachment)))