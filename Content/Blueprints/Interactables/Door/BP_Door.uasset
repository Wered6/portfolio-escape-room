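; BP_Door is an interactable door that swings open on press, or jiggles when locked.
; A press runs the parent logic, then checks LockComponent to play either the restartable TryOpen timeline or the Open timeline, which first disables further interaction.
; Both timelines drive door yaw and handle roll from curves scaled by angle or strength variables.
; It also supplies WidgetAttachment as the widget's attachment component.
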(event EventInteractPressTriggered
  (|CallParentFunction)
  (if (Variables|/Script/EscapeRoom.ERLockComponent|GetbIsLocked (Variables|Default|GetLockComponent))
    (bind (_direction _doortryrotation _handlerotation) (Timeline|TryOpen PlayFromStart)
      (:Update
        (Transformation|SetRelativeRotation (Variables|Default|GetDoorMesh) (Math|Rotator|MakeRotator 0.0 0.0 (* _doortryrotation (Variables|ER|Door|GetDoorTryRotateStr) -1.0)) false false)
        (Transformation|SetRelativeRotation (Variables|Default|GetHandleMesh) (Math|Rotator|MakeRotator (* _handlerotation (Variables|ER|Door|GetHandleRotationAngle) -1.0) 0.0 0.0) false false)))
    (else
      (Class|ERInteractInterface|SetCanInteract false)
      (bind (_direction_2 _doorrotation _handlerotation_2) (Timeline|Open Play)
        (:Update
          (Transformation|SetRelativeRotation (Variables|Default|GetDoorMesh) (Math|Rotator|MakeRotator 0.0 0.0 (* _doorrotation (Variables|ER|Door|GetDoorRotationAngle) -1.0)) false false)
          (Transformation|SetRelativeRotation (Variables|Default|GetHandleMesh) (Math|Rotator|MakeRotator (* _handlerotation_2 (Variables|ER|Door|GetHandleRotationAngle) -1.0) 0.0 0.0) false false))))))

(fn ConstructionScript)

(fn GetWidgetAttachmentComponent
  (return (Variables|Default|GetWidgetAttachment)))